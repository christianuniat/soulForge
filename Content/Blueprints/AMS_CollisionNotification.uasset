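; Anim notify state that turns a weapon animation window into a lethal hit check against ghosts.
; Each notify tick runs a multi sphere trace for objects between the mesh's WeaponBase and WeaponTip sockets.
; Hit actors are cast to BP_Ghost_Actor or, failing that, BP_GhostSeeker, and OnDeath is called directly on a match, with no damage step.
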(fn `Received_NotifyTick`
  (params (MeshComp :type "SkeletalMeshComponent Object Reference") (Animation :type "AnimSequenceBase Object Reference") (FrameDeltaTime :type "Float (single-precision)") (EventReference :type "AnimNotifyEventReference Structure (by ref)"))
  (returns (ReturnValue :type Boolean))
  (bind _outhits (`KismetSystemLibrary.SphereTraceMultiForObjects` :`WorldContextObject` MeshComp :`Start` (`SceneComponent.GetSocketLocation` MeshComp "WeaponBase") :`End` (`SceneComponent.GetSocketLocation` MeshComp "WeaponTip") :`Radius` 20.0 :`ObjectTypes` (`|MakeArray` "ObjectTypeQuery1" "ObjectTypeQuery2" "ObjectTypeQuery3" "ObjectTypeQuery4" "ObjectTypeQuery5" "ObjectTypeQuery6" :!type "EObjectTypeQuery Enum") :`DrawTime` 0.5))
  (if true
    (for _array_element _outhits
      (bind (_bblockinghit _binitialoverlap _time _distance _location _impactpoint _normal _impactnormal _physmat _hitactor) (`GameplayStatics.BreakHitResult` _array_element))
      (bind _asbp_ghost_actor (cast `/Game/Characters/Ghost/BP_Ghost_Actor` _hitactor)
        (:`then`
          (`/Game/Characters/Ghost/BP_Ghost_Actor.OnDeath` _asbp_ghost_actor))
        (:`CastFailed`
          (bind _asbp_ghost_seeker (cast `/Game/Characters/Ghost/BP_GhostSeeker` _hitactor))
          (`/Game/Characters/Ghost/BP_GhostSeeker.OnDeath` _asbp_ghost_seeker))))
    (return false)))