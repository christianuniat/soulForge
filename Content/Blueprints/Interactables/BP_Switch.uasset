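; A pressable switch actor that notifies other objects through its OnButtonPressed event dispatcher.
; The Interaction event snaps the Cylinder mesh to a fixed relative position and fires the dispatcher, with no reset in this graph.
; The Construction Script pushes the radius, line thickness and color from the Interactable settings into the Sphere of its BP_SwitchInteractable child actor.
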(event `/Game/Blueprints/Interactables/BPI_Interactables.Interaction`
  (`SceneComponent.K2_SetRelativeLocation` (`self.Cylinder`) (0.0 0.0 50.0) false false)
  (`self.OnButtonPressed`))

(fn `UserConstructionScript`
  (bind (_interactable_radios _interactable_linethickness _interactable_color) (break `/Game/Blueprints/Interactables/S_Interactable` (`self.Interactable`)))
  (bind _asbp_switch_interactable (cast `/Game/Blueprints/Interactables/BP_SwitchInteractable` (`ChildActorComponent.ChildActor` (`self.BP_SwitchInteractable`))))
  (bind _sphere (`/Game/Blueprints/Interactables/BP_SwitchInteractable.Sphere` _asbp_switch_interactable))
  (`SphereComponent.SetSphereRadius` _sphere _interactable_radios true)
  (`ShapeComponent.SetLineThickness` _sphere _interactable_linethickness)
  (set `ShapeComponent.ShapeColor` _interactable_color _sphere))