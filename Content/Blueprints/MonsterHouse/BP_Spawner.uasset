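; Monster House spawner actor that produces ghost enemies once a trigger starts the event.
; On BeginPlay it binds its MonsterHouse event to the MonsterHouseStart dispatcher of every BP_Trigger in the level.
; The event sets Active and spawns BP_GhostSeeker every two seconds at an offset from its PointLight, with nothing here clearing the flag.
; A separate MonsterHouse function graph spawns a single BP_Ghost_Actor at the same offset.
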(event `self.ReceiveBeginPlay`
  (bind _outactors (`GameplayStatics.GetAllActorsOfClass` "/Game/Blueprints/MonsterHouse/BP_Trigger.BP_Trigger_C"))
  (for _array_element _outactors
    (add `/Game/Blueprints/MonsterHouse/BP_Trigger.MonsterHouse Start` _array_element (delegate `Monster House`))))

(event `Monster House`
  (bind _returnvalue (`SceneComponent.K2_GetComponentToWorld` (`self.PointLight`)))
  ; Spawning
  (set `self.Active` true)
  (if (`self.Active`) :!label _label
    (`|SpawnActorFromClass` "/Game/Characters/Ghost/BP_GhostSeeker.BP_GhostSeeker_C" (`KismetMathLibrary.MakeTransform` (`KismetMathLibrary.MakeVector` (+ (.x (.location _returnvalue)) 100.0) (.y (.location _returnvalue)) (- (.z (.location _returnvalue)) 300.0)) (.rotation _returnvalue) (.scale _returnvalue)) "Undefined" "MultiplyWithRoot" null null)
    (`KismetSystemLibrary.Delay` 2.0)
    (goto _label)))

(fn `MonsterHouse`
  (bind _returnvalue (`SceneComponent.K2_GetComponentToWorld` (`self.PointLight`)))
  (set `self.Active` true)
  (if (`self.Active`)
    (`|SpawnActorFromClass` "/Game/Characters/Ghost/BP_Ghost_Actor.BP_Ghost_Actor_C" (`KismetMathLibrary.MakeTransform` (`KismetMathLibrary.MakeVector` (+ (.x (.location _returnvalue)) 100.0) (.y (.location _returnvalue)) (- (.z (.location _returnvalue)) 300.0)) (.rotation _returnvalue) (.scale _returnvalue)) "Undefined" "MultiplyWithRoot" null null)))

(fn `UserConstructionScript`)